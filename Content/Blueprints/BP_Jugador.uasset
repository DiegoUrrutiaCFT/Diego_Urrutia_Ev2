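; BP_Jugador is the player character, handling movement, jumping, mouse look and projectile shooting.
; Input axes drive control-rotation-relative movement and camera, while firing on button release spawns BP_proyectil at the Disparador transform and spends ammo, and reload restores it to MunicionTotal, with print-string feedback.
; BeginPlay adds the WBP_UI widget to the player screen, and the Morir event opens the EscenaEvaluacion level when VidaActual reaches zero.
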(event `Morir`
  (if (<= (`self.VidaActual`) 0.0)
    (`GameplayStatics.OpenLevel` "EscenaEvaluacion")))

(event `self.ReceiveBeginPlay`
  ;[0.1077 0.5404 1] Agregar UI
  (bind _returnvalue (`|CreateWidget` "/Game/Blueprints/WBP_UI.WBP_UI_C"))
  (`UserWidget.AddToPlayerScreen` _returnvalue 0))

(event `InputAxis|Movimiento Hacia Adelante y Atrasç`
  (params (AxisValue :type "Float (single-precision)"))
  (bind (_returnvalue_roll _returnvalue_pitch _returnvalue_yaw) (`KismetMathLibrary.BreakRotator` (`self.GetControlRotation`)))
  ;[1 0.1927 0.1927] Movimiento
  (`self.AddMovementInput` (`KismetMathLibrary.GetForwardVector` (`KismetMathLibrary.MakeRotator` 0.0 0.0 _returnvalue_yaw)) AxisValue))

(event `InputAction|Salto Player`
  (params (Key :type "Key Structure"))
  ;[1 0.1667 0.1667] Salto
  (:`Pressed`
    (`self.Jump`))
  (:`Released`
    (`self.StopJumping`)))

(event `InputAxis|Movimiento Izquierda y Derecha`
  (params (AxisValue :type "Float (single-precision)"))
  (bind (_returnvalue_roll _returnvalue_pitch _returnvalue_yaw) (`KismetMathLibrary.BreakRotator` (`self.GetControlRotation`)))
  ;[1 0.1927 0.1927] Movimiento
  (`self.AddMovementInput` (`KismetMathLibrary.GetRightVector` (`KismetMathLibrary.MakeRotator` _returnvalue_roll 0.0 _returnvalue_yaw)) AxisValue))

(event `InputAction|Disparo`
  (params (Key :type "Key Structure"))
  ;[0.8594 0.6 0] LOGICA DISPARO
  (:`Released`
    (if (> (`self.MunicionActual`) 0)
      (`|SpawnActorFromClass` "/Game/Blueprints/BP_proyectil.BP_proyectil_C" (`SceneComponent.K2_GetComponentToWorld` (`self.disparador`)) "Undefined" "OverrideRootScale" null null)
      (set `self.MunicionActual` (- (`self.MunicionActual`) 1))
      (`KismetSystemLibrary.PrintString` "DISPARO")
      (else
        (`KismetSystemLibrary.PrintString` "SIN MUNICION, RECARGA")))))

(event `InputAxis|Raton Izquierda y Derecha`
  (params (AxisValue :type "Float (single-precision)"))
  ;[1 0.2344 0.2344] Control Mouse
  (`self.AddControllerYawInput` AxisValue))

(event `InputAction|Recarga`
  (params (Key :type "Key Structure"))
  ;[0.8594 0.6 0] LOGICA DISPARO
  (:`Released`
    (if (< (`self.MunicionActual`) (`self.MunicionTotal`))
      (set `self.MunicionActual` (`self.MunicionTotal`))
      (`KismetSystemLibrary.PrintString` "HAS RECARGADO")
      (else
        (`KismetSystemLibrary.PrintString` "YA TIENES LA MUNICION MAXIMA")))))

(event `InputAxis|Raton Arriba y Abajo`
  (params (AxisValue :type "Float (single-precision)"))
  ;[1 0.2344 0.2344] Control Mouse
  (`self.AddControllerPitchInput` AxisValue))

(fn `UserConstructionScript`)