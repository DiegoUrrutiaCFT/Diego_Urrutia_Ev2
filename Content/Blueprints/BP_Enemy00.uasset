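; BP_Enemy00 is a basic enemy that wanders, chases what it sees and can be killed by stomp or projectile.
; Patrulla slowly walks to random nearby reachable points, re-calling itself after a pause, while PawnSensing issues a move toward any seen pawn.
; Overlapping Debilidad bounces BP_Jugador and destroys the enemy, as does BP_proyectil hitting the mesh.
; Ataque damages and bounces the player, calling GameOver when health drops below zero.
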(event `self.ReceiveBeginPlay`
  ;[1 1 1] Sistema de Patrulla NPC
  (`self.Patrulla`))

(event `Patrulla`
  ;[1 1 1] Sistema de Patrulla NPC
  (set `CharacterMovementComponent.MaxWalkSpeed` 100.0 (`self.CharacterMovement`))
  (bind _output_get (set `self.Random Location` (`NavigationSystemV1.K2_GetRandomReachablePointInRadius` (`self.K2_GetActorLocation`) 300.0 null null)))
  (`|AIMoveTo` self _output_get null 10.0
    (:`OnSuccess`
      (`KismetSystemLibrary.Delay` 3.0)
      (`self.Patrulla`))
    (:`OnFail`
      (`KismetSystemLibrary.Delay` 3.0)
      (`self.Patrulla`))))

(event `self.Debilidad.OnComponentBeginOverlap`
  (params (OverlappedComponent :type "PrimitiveComponent Object Reference") (OtherActor :type "Actor Object Reference") (OtherComp :type "PrimitiveComponent Object Reference") (OtherBodyIndex :type Integer) (bFromSweep :type Boolean) (SweepResult :type "HitResult Structure (by ref)"))
  ;[0.2277 0.4807 1] FUNCION DE DAÑO Y MUERTE ENEMIGO
  (bind _asbp_jugador (cast `/Game/Blueprints/BP_Jugador` OtherActor))
  (`self.Jump` _asbp_jugador)
  (`self.K2_DestroyActor`))

(event `self.Ataque.OnComponentBeginOverlap`
  (params (OverlappedComponent :type "PrimitiveComponent Object Reference") (OtherActor :type "Actor Object Reference") (OtherComp :type "PrimitiveComponent Object Reference") (OtherBodyIndex :type Integer) (bFromSweep :type Boolean) (SweepResult :type "HitResult Structure (by ref)"))
  ;[0.2277 0.4807 1] FUNCION DE DAÑO Y MUERTE ENEMIGO
  (bind _asbp_jugador (cast `/Game/Blueprints/BP_Jugador` OtherActor))
  (set `self.As BP Jugador` _asbp_jugador)
  (set `/Game/Blueprints/BP_Jugador.VidaActual` (- (`/Game/Blueprints/BP_Jugador.VidaActual` _asbp_jugador) 500.0) _asbp_jugador)
  (`self.Jump` _asbp_jugador)
  (if (< (`/Game/Blueprints/BP_Jugador.VidaActual` _asbp_jugador) 0.0)
    (bind _asbp_jugador_2 (cast `/Game/Blueprints/BP_Jugador` (`self.As BP Jugador`)))
    (`/Game/Blueprints/BP_Jugador.GameOver` _asbp_jugador_2)))

(event `self.SkeletalMesh.OnComponentBeginOverlap`
  (params (OverlappedComponent :type "PrimitiveComponent Object Reference") (OtherActor :type "Actor Object Reference") (OtherComp :type "PrimitiveComponent Object Reference") (OtherBodyIndex :type Integer) (bFromSweep :type Boolean) (SweepResult :type "HitResult Structure (by ref)"))
  (cast `/Game/Blueprints/BP_proyectil` OtherActor)
  (`self.K2_DestroyActor`))

(event `self.PawnSensing.OnSeePawn`
  (params (Pawn :type "Pawn Object Reference"))
  (`|AIMoveTo` self (0.0 0.0 0.0) Pawn))

(fn `UserConstructionScript`)