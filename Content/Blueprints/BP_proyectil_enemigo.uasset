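; BP_proyectil_enemigo is an enemy projectile that damages the player on contact.
; Its Sphere1 overlap casts to BP_Jugador, subtracts a fixed amount directly from VidaActual and makes the player jump.
; It spawns a particle effect at the player's location, then calls DestroyActor twice on itself.
; The emitter is deactivated immediately, with its component destruction placed behind a short Delay that follows the actor's own destruction.
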(event `self.Sphere1.OnComponentBeginOverlap`
  (params (OverlappedComponent :type "PrimitiveComponent Object Reference") (OtherActor :type "Actor Object Reference") (OtherComp :type "PrimitiveComponent Object Reference") (OtherBodyIndex :type Integer) (bFromSweep :type Boolean) (SweepResult :type "HitResult Structure (by ref)"))
  ;[0.156 0.3986 1] Sistema Particulas y Daño a JUGADOR
  (bind _asbp_jugador (cast `/Game/Blueprints/BP_Jugador` OtherActor))
  (set `/Game/Blueprints/BP_Jugador.VidaActual` (- (`/Game/Blueprints/BP_Jugador.VidaActual` _asbp_jugador) 20.0) _asbp_jugador)
  (`Character.Jump` _asbp_jugador)
  (bind _returnvalue (`GameplayStatics.SpawnEmitterAtLocation` "/Engine/Tutorial/SubEditors/TutorialAssets/TutorialParticleSystem.TutorialParticleSystem" (`self.K2_GetActorLocation` _asbp_jugador) (struct) (1.0 1.0 1.0) false))
  (`self.K2_DestroyActor`)
  (`self.K2_DestroyActor`)
  (`ActorComponent.Deactivate` _returnvalue)
  (`KismetSystemLibrary.Delay` 0.1)
  (`ActorComponent.K2_DestroyComponent` _returnvalue))

(fn `UserConstructionScript`)